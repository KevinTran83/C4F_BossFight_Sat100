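; Player character Blueprint that handles basic movement, jumping and camera look through Enhanced Input.
; BeginPlay adds the IMC_BossFighter mapping context to the local player's input subsystem.
; Movement follows SpringArm vectors, with IA_Forward using the right vector and IA_Right using the forward vector, crossed relative to their names.
; IA_Look drives controller yaw and pitch, and IA_Jump starts and stops jumping.
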(event `self.ReceiveBeginPlay`
  (bind _asplayer_controller (cast `PlayerController` (`self.GetController`)))
  (`EnhancedInputSubsystemInterface.AddMappingContext` (pcsubsystem `EnhancedInputLocalPlayerSubsystem` _asplayer_controller) "/Game/C4F_BossFight/Inputs/IMC_BossFighter.IMC_BossFighter" 0 (struct)))

(event `self.ReceiveTick`
  (params (DeltaSeconds :type "Float (single-precision)")))

(event `EnhancedInput|/Game/C4F_BossFight/Inputs/IA_Forward`
  (params (ActionValue :type "Float (double-precision)") (ElapsedSeconds :type "Float (double-precision)") (TriggeredSeconds :type "Float (double-precision)") (InputAction :type "InputAction Object Reference" :default "/Game/C4F_BossFight/Inputs/IA_Forward.IA_Forward"))
  ;[1 1 1] Movement
  (:`Triggered`
    (`self.AddMovementInput` (`SceneComponent.GetRightVector` (`self.SpringArm`)) ActionValue)))

(event `EnhancedInput|/Game/C4F_BossFight/Inputs/IA_Right`
  (params (ActionValue :type "Float (double-precision)") (ElapsedSeconds :type "Float (double-precision)") (TriggeredSeconds :type "Float (double-precision)") (InputAction :type "InputAction Object Reference" :default "/Game/C4F_BossFight/Inputs/IA_Right.IA_Right"))
  ;[1 1 1] Movement
  (:`Triggered`
    (`self.AddMovementInput` (`SceneComponent.GetForwardVector` (`self.SpringArm`)) ActionValue)))

(event `EnhancedInput|/Game/C4F_BossFight/Inputs/IA_Jump`
  (params (ActionValue :type Boolean) (ElapsedSeconds :type "Float (double-precision)") (TriggeredSeconds :type "Float (double-precision)") (InputAction :type "InputAction Object Reference" :default "/Game/C4F_BossFight/Inputs/IA_Jump.IA_Jump"))
  ;[1 1 1] Jumping
  (:`Triggered`
    (`self.Jump`))
  (:`Completed`
    (`self.StopJumping`)))

(event `EnhancedInput|/Game/C4F_BossFight/Inputs/IA_Look`
  (params (ActionValue :type "Vector2D Structure") (ElapsedSeconds :type "Float (double-precision)") (TriggeredSeconds :type "Float (double-precision)") (InputAction :type "InputAction Object Reference" :default "/Game/C4F_BossFight/Inputs/IA_Look.IA_Look"))
  (:`Triggered`
    (`self.AddControllerYawInput` ActionValue_X)
    (`self.AddControllerPitchInput` ActionValue_Y)))

(fn `UserConstructionScript`)