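; BP_MotionDetector reports whether the Character that owns it is actively moving.
; On BeginPlay it casts its owner to Character and caches that character and its movement component, doing nothing further if the cast fails.
; IsMoving returns true only when horizontal velocity exceeds MinWalkSpeed and current acceleration is non-zero, so coasting without acceleration does not count as moving.
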(event `self.ReceiveBeginPlay`
  (bind _ascharacter (cast `Character` (`self.GetOwner`)))
  (bind _output_get (set `self.Character` _ascharacter))
  (set `self.Movement` (`Character.CharacterMovement` _output_get)))

(fn `IsMoving`
  (returns (`Is Moving` :type Boolean))
  (bind _movement (`self.Movement`))
  (return (and (> (`KismetMathLibrary.VSizeXY` (`MovementComponent.Velocity` _movement)) (`self.MinWalkSpeed`)) (!= (`CharacterMovementComponent.GetCurrentAcceleration` _movement) (0.0 0.0 0.0)))))